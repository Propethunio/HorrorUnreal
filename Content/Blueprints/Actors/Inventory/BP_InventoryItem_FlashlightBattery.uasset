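; Inventory item actor for a flashlight battery that recharges the player's flashlight when used.
; UseItem checks the player's flashlight component and, if the battery is below its maximum, replenishes it by the item's battery amount.
; It records whether the use succeeded, so using it on a full battery fails.
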(event `self.UseItem`
  (bind _bpc_flashlight (`/Game/Blueprints/Game/Level1/L1_Character.BPC_Flashlight` (`self.PlayerRef`)))
  (if (< (`/Game/Blueprints/ActorComponents/BPC_Flashlight.CurrentBatteryLevel` _bpc_flashlight) (`/Game/Blueprints/ActorComponents/BPC_Flashlight.MaxBatteryLevel` _bpc_flashlight))
    (`/Game/Blueprints/ActorComponents/BPC_Flashlight.ReplenishBattery` _bpc_flashlight (`self.BatteryAmount`))
    (set `self.UseItemSuccess` true)
    (else
      (set `self.UseItemSuccess` false))))

(fn `UserConstructionScript`
  (`parent.UserConstructionScript`))