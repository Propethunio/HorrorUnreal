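; BPC_Movement is an actor component that handles walking, sprinting and crouching for the player, including sprint stamina.
; It sets the character's max walk speed per state and calls L1_Character to shorten or lengthen the capsule when crouching.
; Looping function-name timers drain stamina while sprinting and moving, then regenerate it after a retriggerable delay following a sprint stop.
; Starting a sprint cancels crouch, and sprinting stops when stamina runs out or movement nearly ceases.
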(event `StartCrouch`
  ;[1 1 1] Start Crouching
  (`KismetSystemLibrary.K2_ClearTimer` null "SprintTImer")
  (`self.SetPlayerMaxWalkSpeed` (`self.CrouchSpeed`))
  (`/Game/Blueprints/Game/Level1/L1_Character.ShortenPlayerCapsule` (cast `/Game/Blueprints/Game/Level1/L1_Character` (`self.PlayerRef`) :!pure true))
  (set `self.IsCrouching` true))

(event `StartSprint`
  ;[1 1 1] Start Sprinting
  (if (`self.IsCrouching`)
    (`self.EndCrouch`))
  (if (and (> (`self.CurrentStamina`) (`self.MinStamina`)) (> (`KismetMathLibrary.VSize` (`Actor.GetVelocity` (`self.PlayerRef`))) 10.0))
    (`KismetSystemLibrary.K2_ClearTimer` null "RegenerateStamina")
    (`self.SetPlayerMaxWalkSpeed` (`self.SprintSpeed`))
    (`KismetSystemLibrary.K2_SetTimer` null "SprintTimer" 0.1 true)))

(event `EndCrouch`
  ;[1 1 1] End Crouching
  (`self.SetPlayerMaxWalkSpeed` (`self.WalkSpeed`))
  (`/Game/Blueprints/Game/Level1/L1_Character.LenghtenPlayerCapsule` (cast `/Game/Blueprints/Game/Level1/L1_Character` (`self.PlayerRef`) :!pure true))
  (set `self.IsCrouching` false))

(event `SprintTimer`
  ;[1 1 1] Sprint Timer
  (if (> (`KismetMathLibrary.VSize` (`Actor.GetVelocity` (`self.PlayerRef`))) 10.0)
    (set `self.CurrentStamina` (`KismetMathLibrary.FClamp` (- (`self.CurrentStamina`) 1.0) (`self.MinStamina`) (`self.MaxStamina`)))
    (if (<= (`self.CurrentStamina`) (`self.MinStamina`))
      (`self.StopSprint`))
    (else
      (`self.StopSprint`))))

(event `StopSprint`
  ;[1 1 1] Stop Sprint
  (if (not (`self.IsCrouching`))
    (`KismetSystemLibrary.K2_ClearTimer` null "SprintTImer")
    (`self.SetPlayerMaxWalkSpeed` (`self.WalkSpeed`))
    (`KismetSystemLibrary.RetriggerableDelay` 2.0)
    (if (not (`KismetSystemLibrary.K2_IsTimerActive` null "SprintTimer"))
      (`KismetSystemLibrary.K2_SetTimer` null "RegenerateStamina" 0.03 true))))

(event `RegenerateStamina`
  ;[1 1 1] Regenerate Stamina
  (set `self.CurrentStamina` (`KismetMathLibrary.FClamp` (+ (`self.CurrentStamina`) 1.0) (`self.MinStamina`) (`self.MaxStamina`)))
  (if (>= (`self.CurrentStamina`) (`self.MaxStamina`))
    (`KismetSystemLibrary.K2_ClearTimer` null "RegenerateStamina")))

(fn `Initialize`
  (params (Character :type "Character Object Reference"))
  (set `self.PlayerRef` Character)
  (set `CharacterMovementComponent.MaxWalkSpeed` (`self.WalkSpeed`) (`Character.CharacterMovement` (`self.PlayerRef`))))

(fn `SetPlayerMaxWalkSpeed`
  (params (`Max Walk Speed` :type "Float (single-precision)"))
  (set `CharacterMovementComponent.MaxWalkSpeed` `Max Walk Speed` (`Character.CharacterMovement` (`self.PlayerRef`))))